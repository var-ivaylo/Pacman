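; Coin pickup actor that a Default_Character collects by overlapping it.
; On overlap it calls LightUp on the character, plays a pickup sound at its location, reports the pickup to Default_GameMode via PickupCoin, then destroys itself.
; Tick spins the coin around yaw at RotationRate, scaled by delta time and with pitch and roll held at zero.
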(event EventBeginPlay)

(event EventActorBeginOverlap
  (params (OtherActor :type Actor%20Object%20Reference))
  (bind _asdefault_character (Utilities|Casting|CastToDefault_Character OtherActor))
  (Default|LightUp _asdefault_character)
  (Audio|PlaySoundatLocation "/Game/Audio/CoinPickup.CoinPickup" (Transformation|GetActorLocation) 0.25)
  (bind _asdefault_game_mode (Utilities|Casting|CastToDefault_GameMode (Game|GetGameMode)))
  (Default|PickupCoin _asdefault_game_mode)
  (Actor|DestroyActor))

(event EventTick
  (params (DeltaSeconds :type Float%20%28single-precision%29))
  (Transformation|SetActorRotation (Class|KismetMathLibrary|MakeRot 0.0 (+ (* DeltaSeconds (Variables|Default|GetRotationRate)) (.Yaw (Class|KismetMathLibrary|BreakRot (Transformation|GetActorRotation)))) 0.0)))

(fn ConstructionScript)